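; Level manager that spawns a wave of enemies when play begins, after a short delay if the player pawn is found.
; SpawnWave spends a DifficultyLevel point budget, subtracting each spawned enemy's StrengthValue until none remains.
; SpawnEnemy places a BP_BasicEnemy at a random X/Z position within the spawn range.
; Enemy type selection is stubbed, so every spawn is a basic enemy.
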(event Custom|Spawn%20Wave
  ;[1 1 1] Spawn Wave of Enemies
  (Variables|Default|SetDiffifultyPointsRemaining (Variables|Default|GetDifficultyLevel))
  (while (> (Variables|Default|GetDiffifultyPointsRemaining) 0)
    (switch int (Math|Random|RandomInteger 0)
      (:Default
        _)
      (:0
        _))
    (bind _enemy_found (CallFunction|SpawnEnemy "NewEnumerator0"))
    (Variables|Default|SetDiffifultyPointsRemaining (- (Variables|Default|GetDiffifultyPointsRemaining) (Variables|/Game/Blueprints/BP_BasicEnemy.BP_BasicEnemy_C|GetStrength%20Value _enemy_found)))))

(event EventBeginPlay
  ;[1 1 1] Initialization
  (Utilities|Casting|CastToBP_PlayerChar (Game|Player|GetPlayerPawn 0)
    (:then
      (Variables|Default|SetPlayer%20Character 0)
      (Utilities|FlowControl|Delay 4.0)
      (CallFunction|SpawnWave))
    (:CastFailed
      (CallFunction|SpawnWave)
      (Development|PrintString "Could Not Identify Player" true true "(R=1.000000,G=0.000000,B=0.179544,A=1.000000)"))))

(event EventTick
  (params (DeltaSeconds :type Float%20%28single-precision%29))
  ;[1 1 1] Spawn Wave of Enemies
)

(fn ConstructionScript)

(fn SpawnEnemy
  (params (Enemy%20Type :type EnemyTypes%20Enum :default "NewEnumerator0"))
  (bind _spawn_range_min (Variables|Default|GetSpawn%20Range%20Min))
  (bind _spawn_range_max (Variables|Default|GetSpawn%20Range%20Max))
  (switch Utilities|FlowControl|Switch|SwitchonEnemyTypes Enemy%20Type
    (:NewEnumerator0
      (bind _returnvalue (Game|SpawnActorfromClass "/Game/Blueprints/BP_BasicEnemy.BP_BasicEnemy_C" (Math|Transform|MakeTransform (Math|Vector|MakeVector (Math|Random|RandomFloatinRange (.x _spawn_range_min) (.x _spawn_range_max)) 0.0 (Math|Random|RandomFloatinRange (.y _spawn_range_min) (.y _spawn_range_max))) "0.000000,180.000000,0.000000" "1.000000,1.000000,1.000000") "Undefined" "MultiplyWithRoot" 0 1 0))
      (return _returnvalue))))