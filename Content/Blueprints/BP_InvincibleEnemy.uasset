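; BP_InvincibleEnemy is an enemy whose BulletDamage event has no logic, so bullet hits do nothing to it.
; On BeginPlay it starts the Parabola timeline, which replays after a short delay each time it finishes.
; Each update steps the Cube's relative X down by EnemySpeed and maps the curve value onto its Z, sweeping it vertically while it advances.
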(event Custom|Move%20Up%20and%20Down
  (bind _cube (Variables|Default|GetCube))
  (bind _position (Timeline|Parabola PlayFromStart)
    (:Update
      (Transformation|SetRelativeLocation _cube (Math|Vector|MakeVector (- (.X (Math|Vector|BreakVector (Variables|/Script/Engine.SceneComponent|GetRelativeLocation _cube))) (Variables|Default|GetEnemy%20Speed)) 0.0 (Math|Float|MapRangeClamped _position -1.0 1.0 -6.5e+02 6.5e+02)) false false))
    (:Finished
      (Utilities|FlowControl|Delay 0.2)
      (Timeline|Parabola PlayFromStart))))

(event EventBeginPlay
  (CallFunction|MoveUpandDown))

(event Collision|EventActorBeginOverlap
  (params (OtherActor :type Actor%20Object%20Reference)))

(event EventTick
  (params (DeltaSeconds :type Float%20%28single-precision%29)))

(event EventBulletDamage)

(fn ConstructionScript)