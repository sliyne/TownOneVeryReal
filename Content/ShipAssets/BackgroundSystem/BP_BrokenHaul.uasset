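; BP_BrokenHaul is a drifting background prop, apparently a piece of broken ship hull, in the ship BackgroundSystem.
; On BeginPlay it takes a random rotation and teleports to a fixed far X and Y with a random height.
; Each Tick it moves a fixed step along negative X with a slow tumble on all axes, independent of delta time, and destroys itself past the far X limit.
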(event EventBeginPlay
  (bind _defaultsceneroot (Variables|Default|GetDefaultSceneRoot))
  (Transformation|SetWorldRotation _defaultsceneroot (Math|Random|RandomRotator true) false false)
  (Transformation|SetWorldLocation _defaultsceneroot (Math|Vector|MakeVector 2e+04 -7.19e+03 (Math|Random|RandomFloatinRange -4.17e+03 1.58e+03)) false true))

(event Collision|EventActorBeginOverlap
  (params (OtherActor :type Actor%20Object%20Reference)))

(event EventTick
  (params (DeltaSeconds :type Float%20%28single-precision%29))
  (bind _defaultsceneroot (Variables|Default|GetDefaultSceneRoot))
  (bind _returnvalue (Transformation|GetWorldRotation _defaultsceneroot))
  (bind _returnvalue_2 (Transformation|GetWorldLocation _defaultsceneroot))
  (bind (_roll _pitch _yaw) (Math|Rotator|BreakRotator _returnvalue))
  (bind (_x _y _z) (Math|Vector|BreakVector _returnvalue_2))
  (if (< _x -2e+04)
    (Actor|DestroyActor self)
    (else
      (Transformation|SetWorldLocation _defaultsceneroot (Math|Vector|MakeVector (+ _x -6.0) _y _z) false false)
      (Transformation|SetWorldRotation _defaultsceneroot (Math|Rotator|MakeRotator (+ _roll 0.01) (+ _pitch 0.01) (+ _yaw 0.01)) false false))))

(fn ConstructionScript)