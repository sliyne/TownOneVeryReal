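; BP_BGSpawner is a background spawner actor that endlessly spawns rocks, docks and broken hauls for the ship background system.
; Tick drives three independent DoOnce gates, each spawning its class and then resetting after a random delay, with rocks recurring most often.
; Every spawn uses the same fixed, far-off world transform, so this Blueprint does no placement of its own.
; The BeginPlay delay leads to nothing and does not hold back spawning.
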(event EventBeginPlay
  (Utilities|FlowControl|Delay 2.0))

(event Collision|EventActorBeginOverlap
  (params (OtherActor :type Actor%20Object%20Reference)))

(event EventTick
  (params (DeltaSeconds :type Float%20%28single-precision%29))
  (Utilities|FlowControl|Sequence
    (:then_0
      (Utilities|FlowControl|DoOnce false :!label _label
        (:Completed
          (Game|SpawnActorfromClass "/Game/ShipAssets/BackgroundSystem/BP_Rocks.BP_Rocks_C" (Math|Transform|MakeTransform "90000.000000,90000.000000,90000.000000") "Undefined" "MultiplyWithRoot" 0 0)
          (Utilities|FlowControl|Delay (Math|Random|RandomFloatinRange 1.0 6.0))
          (goto _label Reset))))
    (:then_1
      (Utilities|FlowControl|DoOnce false :!label _label_2
        (:Completed
          (Game|SpawnActorfromClass "/Game/ShipAssets/BackgroundSystem/BP_Dock.BP_Dock_C" (Math|Transform|MakeTransform "90000.000000,90000.000000,90000.000000") "Undefined" "MultiplyWithRoot" 0 0)
          (Utilities|FlowControl|Delay (Math|Random|RandomFloatinRange 1e+01 2e+01))
          (goto _label_2 Reset))))
    (:then_2
      (Utilities|FlowControl|DoOnce false :!label _label_3
        (:Completed
          (Game|SpawnActorfromClass "/Game/ShipAssets/BackgroundSystem/BP_BrokenHaul.BP_BrokenHaul_C" (Math|Transform|MakeTransform "90000.000000,90000.000000,90000.000000") "Undefined" "MultiplyWithRoot" 0 0)
          (Utilities|FlowControl|Delay (Math|Random|RandomFloatinRange 15.0 33.0))
          (goto _label_3 Reset))))))

(fn ConstructionScript)