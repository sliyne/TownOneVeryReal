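; BP_Rocks is a scrolling background rock actor for the ship's background system.
; On BeginPlay it gets a random rotation, scale and negative speed, then teleports to a fixed spawn X and Y with a random height.
; Each Tick it drifts along negative X at that per-frame speed, not scaled by delta time, while slowly tumbling, and destroys itself once past a far X limit.
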(event EventBeginPlay
  (bind _defaultsceneroot (Variables|Default|GetDefaultSceneRoot))
  (Transformation|SetWorldRotation _defaultsceneroot (Math|Random|RandomRotator true) false false)
  (Transformation|SetWorldScale3D _defaultsceneroot (Math|Conversions|ToVector(Float) (Math|Random|RandomFloatinRange 1.0 4.4)))
  (Variables|Default|SetSpeed (* (Math|Random|RandomFloatinRange 9.0 1e+01) -1.0))
  (Transformation|SetWorldLocation (Variables|Default|GetDefaultSceneRoot) (Math|Vector|MakeVector 6.66e+03 -2.55e+03 (Math|Random|RandomFloatinRange -1.9e+03 1.9e+03)) false true))

(event Collision|EventActorBeginOverlap
  (params (OtherActor :type Actor%20Object%20Reference)))

(event EventTick
  (params (DeltaSeconds :type Float%20%28single-precision%29))
  (bind _defaultsceneroot (Variables|Default|GetDefaultSceneRoot))
  (bind _returnvalue (Transformation|GetWorldRotation _defaultsceneroot))
  (bind _returnvalue_2 (Transformation|GetWorldLocation _defaultsceneroot))
  (bind (_roll _pitch _yaw) (Math|Rotator|BreakRotator _returnvalue))
  (bind (_x _y _z) (Math|Vector|BreakVector _returnvalue_2))
  (if (< _x -2e+04)
    (Actor|DestroyActor self)
    (else
      (Transformation|SetWorldLocation _defaultsceneroot (Math|Vector|MakeVector (+ _x (Variables|Default|GetSpeed)) _y _z) false false)
      (Transformation|SetWorldRotation _defaultsceneroot (Math|Rotator|MakeRotator (+ _roll 0.03) (+ _pitch 0.03) (+ _yaw 0.03)) false false))))

(fn ConstructionScript)