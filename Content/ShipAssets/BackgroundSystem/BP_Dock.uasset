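; BP_Dock is a scrolling dock actor for the background system that moves past along the X axis and removes itself.
; On BeginPlay it teleports its root to a fixed start position and randomly picks one of two orientations a half-turn apart.
; Tick steps it toward negative X by a fixed amount per frame, unscaled by delta time, and destroys it past a far threshold.
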(event EventBeginPlay
  (bind _defaultsceneroot (Variables|Default|GetDefaultSceneRoot))
  (Transformation|SetWorldLocation (Variables|Default|GetDefaultSceneRoot) (Math|Vector|MakeVector 3e+03 1e+01 -8.2e+02) false true)
  (if (Math|Random|RandomBool)
    (Transformation|SetWorldRotation _defaultsceneroot "0, 0, 0" false false)
    (else
      (Transformation|SetWorldRotation _defaultsceneroot "0.000000,0.000000,180.000000" false false))))

(event Collision|EventActorBeginOverlap
  (params (OtherActor :type Actor%20Object%20Reference)))

(event EventTick
  (params (DeltaSeconds :type Float%20%28single-precision%29))
  (bind _defaultsceneroot (Variables|Default|GetDefaultSceneRoot))
  (bind _returnvalue (Transformation|GetWorldLocation _defaultsceneroot))
  (bind (_x _y _z) (Math|Vector|BreakVector _returnvalue))
  (if (< _x -1e+04)
    (Actor|DestroyActor self)
    (else
      (Transformation|SetWorldLocation _defaultsceneroot (Math|Vector|MakeVector (+ _x -11.0) _y _z) false false))))

(fn ConstructionScript)