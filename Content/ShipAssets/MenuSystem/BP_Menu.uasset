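; BP_Menu is an actor that sets up the game's menu on BeginPlay.
; It first applies user settings that cap the frame rate and enable VSync, then plays the menu music, keeping a reference to the sound.
; It then creates the Menu_Buttons widget, sets Game and UI input focused on it, shows the mouse cursor and plays the widget's fade-in animation.
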(event Collision|EventActorBeginOverlap
  (params (OtherActor :type Actor%20Object%20Reference)))

(event EventTick
  (params (DeltaSeconds :type Float%20%28single-precision%29)))

(event EventBeginPlay
  (bind _returnvalue (Game|GetPlayerController 0))
  (Utilities|FlowControl|Sequence
    (:then_0
      (bind _returnvalue_2 (Settings|GetGameUserSettings))
      (Class|GameUserSettings|SetFrameRateLimit _returnvalue_2 6e+01)
      (Class|GameUserSettings|SetVSyncEnabled _returnvalue_2 true)
      (Class|GameUserSettings|ApplySettings _returnvalue_2 true))
    (:then_1
      (bind _returnvalue_3 (Audio|SpawnSound2D "/Game/ShipAssets/MenuSystem/MenuMusic.MenuMusic" 1.0 1.0 0.0 0))
      (Variables|Default|SetAudio _returnvalue_3)
      (bind _returnvalue_4 (UserInterface|CreateWidget "/Game/ShipAssets/MenuSystem/Menu_Buttons.Menu_Buttons_C" _returnvalue))
      (bind _output_get (Variables|Default|SetUI_Widget _returnvalue_4))
      (Input|SetInputModeGameandUI _returnvalue _output_get "DoNotLock" true false)
      (UserInterface|Viewport|AddtoViewport _output_get 0)
      (Variables|/Script/Engine.PlayerController|SetbShowMouseCursor _returnvalue true)
      (Components|Animation|PlayAnimation _output_get (Variables|/Game/ShipAssets/MenuSystem/Menu_Buttons.Menu_Buttons_C|GetFadeIn _output_get) 0.0))))

(fn ConstructionScript)