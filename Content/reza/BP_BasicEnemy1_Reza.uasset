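; Basic side-scrolling enemy actor that drifts along negative X while bobbing vertically, firing projectiles as it goes.
; A Timeline started on BeginPlay maps its curve to a height offset around the spawn Z, steps X by EnemySpeed and clamps Z within fixed bounds.
; Tick feeds a random Delay, acting as a repeating timer that spawns BP_EnemyProjectile.
; Any damage caused by a BP_PlayerProjectile destroys the enemy immediately.
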(event Custom|Move%20Up%20and%20Down
  (bind _returnvalue (Transformation|GetActorLocation))
  (bind _returnvalue_2 (Transformation|GetActorLocation))
  ;[1 1 1] Move enemy
  (Variables|Default|SetStarting%20Height (.z (Transformation|GetActorLocation)))
  (bind _position (Timeline|Timeline Play)
    (:Update
      (Transformation|SetActorLocation (Math|Vector|MakeVector (- (.x (Transformation|GetActorLocation)) (Variables|Default|GetEnemy%20Speed)) 0.0 (+ (Math|Float|MapRangeClamped _position -1.0 1.0 -4e+02 4e+02) (Variables|Default|GetStarting%20Height))) false false)
      (if (> (.z _returnvalue_2) 6e+02)
        (Transformation|SetActorLocation (Math|Vector|MakeVector (.x _returnvalue_2) (.y _returnvalue_2) 6e+02) false false)
        (elif (< (.z _returnvalue) -6e+02)
          (Transformation|SetActorLocation (Math|Vector|MakeVector (.x _returnvalue) (.y _returnvalue) -6e+02) false false))))))

(event EventBeginPlay
  (CallFunction|MoveUpandDown))

(event Collision|EventActorBeginOverlap
  (params (OtherActor :type Actor%20Object%20Reference)))

(event EventTick
  (params (DeltaSeconds :type Float%20%28single-precision%29))
  (Utilities|FlowControl|Delay (Math|Random|RandomFloatinRange 1.5 2.5))
  (Game|SpawnActorfromClass "/Game/Blueprints/BP_EnemyProjectile.BP_EnemyProjectile_C" (Math|Transform|MakeTransform (Transformation|GetActorLocation) "0.000000,180.000000,0.000000" "1.000000,1.000000,1.000000") "Undefined" "MultiplyWithRoot" 0 0))

(event Game|Damage|EventAnyDamage
  (params (Damage :type Float%20%28single-precision%29) (DamageType :type Damage%20Type%20Object%20Reference) (InstigatedBy :type Controller%20Object%20Reference) (DamageCauser :type Actor%20Object%20Reference))
  (Utilities|Casting|CastToBP_PlayerProjectile DamageCauser)
  (Actor|DestroyActor))

(fn ConstructionScript)