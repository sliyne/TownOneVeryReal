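; Player Blueprint that moves in the world X/Z plane and fires projectiles.
; On BeginPlay it spawns a separate Camera actor at its own transform, stores it and makes it player 0's view target.
; Horizontal and vertical axis inputs apply fixed-step world offsets, without delta-time scaling or sweep.
; Pressing Fire spawns a BP_PlayerProjectile at the player's transform.
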(event EventBeginPlay
  (bind _returnvalue (Game|SpawnActorfromClass "/Game/Blueprints/Camera.Camera_C" (Transformation|GetActorTransform) "Undefined" "OverrideRootScale" 0 0))
  (bind _output_get (Variables|Default|SetCamera%20Syetem _returnvalue))
  (Game|Player|SetViewTargetwithBlend (Game|GetPlayerController 0) _output_get 0.0 "VTBlend_Linear" 0.0 false))

(event Input|ActionEvents|InputActionFire
  (params (Key :type Key%20Structure))
  (:Pressed
    (Game|SpawnActorfromClass "/Game/Blueprints/BP_PlayerProjectile.BP_PlayerProjectile_C" (Transformation|GetActorTransform) "Undefined" "MultiplyWithRoot" 0 0)))

(event Input|AxisEvents|InputAxisMoveHorizontal
  (params (AxisValue :type Float%20%28single-precision%29))
  (Transformation|AddActorWorldOffset (Math|Vector|MakeVector (* AxisValue 5.0) 0.0 0.0)))

(event Input|AxisEvents|InputAxisMoveVertical
  (params (AxisValue :type Float%20%28single-precision%29))
  (Transformation|AddActorWorldOffset (Math|Vector|MakeVector 0.0 0.0 (* AxisValue 5.0))))

(fn ConstructionScript)